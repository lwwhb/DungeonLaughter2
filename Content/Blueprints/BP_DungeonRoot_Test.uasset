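; BP_DungeonRoot_Test is a test dungeon root that builds a small, hard-wired binary tree of dungeon nodes and enters the dungeon.
; On BeginPlay it initializes the layer 1 root, attaches left and right layer 2 children, then adds a layer 3 left child under the layer 2 left node.
; Each step runs only if the previous one succeeds, so EnterDungeon fires only after the whole tree is built.
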(event EventBeginPlay
  (bind _dungeonnodelayer1root (Variables|Default|GetDungeonNodeLayer1Root))
  (bind _dungeonnodelayer2left (Variables|Default|GetDungeonNodeLayer2Left))
  (bind _returnvalue (Class|DungeonRoot|InitRootDungeonNode _dungeonnodelayer1root))
  (if _returnvalue
    (bind _returnvalue_2 (Class|DungeonRoot|AddLeftDungeonNode _dungeonnodelayer1root _dungeonnodelayer2left))
    (if _returnvalue_2
      (bind _returnvalue_3 (Class|DungeonRoot|AddRightDungeonNode _dungeonnodelayer1root (Variables|Default|GetDungeonNodeLayer2Right)))
      (if _returnvalue_3
        (bind _returnvalue_4 (Class|DungeonRoot|AddLeftDungeonNode _dungeonnodelayer2left (Variables|Default|GetDungeonNodeLayer3Left)))
        (if _returnvalue_4
          (Class|DungeonRoot|EnterDungeon))))))

(event Collision|EventActorBeginOverlap
  (params (OtherActor :type Actor%20Object%20Reference)))

(event EventTick
  (params (DeltaSeconds :type Float%20%28single-precision%29)))

(fn ConstructionScript)